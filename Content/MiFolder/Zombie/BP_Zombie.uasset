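; BP_Zombie is a zombie enemy that chases the player once its detection sphere overlaps BP_FirstPersonCharacter.
; The overlap sets SeePlayer, which is never cleared here, so the chase does not end.
; Each Tick it writes CharacterMovement velocity straight toward the player controller's actor location, without pathfinding, or zeroes it while idle.
; Health is initialized on BeginPlay but not otherwise used.
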(event OnComponentBeginOverlap(Sphere)
  (params (OverlappedComponent :type Primitive%20Component%20Object%20Reference) (OtherActor :type Actor%20Object%20Reference) (OtherComp :type Primitive%20Component%20Object%20Reference) (OtherBodyIndex :type Integer) (bFromSweep :type Boolean) (SweepResult :type Hit%20Result%20Structure%20%28by%20ref%29))
  (Utilities|Casting|CastToBP_FirstPersonCharacter OtherActor)
  (Variables|Default|SetSeePlayer true))

(event EventBeginPlay
  (Variables|Default|SetCurrentHelath (Variables|Default|GetMaxHealth))
  (Variables|Default|SetWalkSpeed 0.0))

(event Collision|EventActorBeginOverlap
  (params (OtherActor :type Actor%20Object%20Reference)))

(event EventTick
  (params (DeltaSeconds :type Float%20%28single-precision%29))
  (if (Variables|Default|GetSeePlayer)
    (Variables|Default|SetWalkSpeed 3e+02)
    (bind _output_get (Variables|Default|SetDir (Math|Vector|Normalize (- (Transformation|GetActorLocation (Game|GetPlayerController 0)) (Transformation|GetWorldLocation (Variables|Collision|GetCapsuleComponent))))))
    (Variables|/Script/Engine.MovementComponent|SetVelocity (Variables|Character|GetCharacterMovement) (* _output_get (Variables|Default|GetWalkSpeed)))
    (else
      (Variables|Default|SetWalkSpeed 0.0)
      (Variables|/Script/Engine.MovementComponent|SetVelocity (Variables|Character|GetCharacterMovement) "0, 0, 0"))))

(fn ConstructionScript)